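; BP_Gun is a gun actor with a Niagara beam and input bindings for shooting and reloading.
; Tick stretches the beam by feeding the distance from the beam to EndPoint into its EndPos X value.
; The beam starts hidden, and AttachGunReceive reveals it and zeroes the emissive brightness on a dynamic material created at BeginPlay.
; Thumb mouse button 2 calls Shoot and R calls Reload, neither defined in this graph.
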(event EventBeginPlay
  (Rendering|SetVisibility (Variables|Default|GetNS_Beam) false false)
  (bind _returnvalue (Rendering|Material|CreateDynamicMaterialInstance (Variables|Default|GetSkeletalMeshComponent) 0 0 "None" :!class /Script/Engine.PrimitiveComponent))
  (Variables|Default|SetGunMat _returnvalue))

(event EventAttachGunReceive
  (Rendering|SetVisibility (Variables|Default|GetNS_Beam) true false)
  (Rendering|Material|SetScalarParameterValue (Variables|Default|GetGunMat) "EmissiveBright" 0.0 :!class /Script/Engine.MaterialInstanceDynamic))

(event EventTick
  (params (DeltaSeconds :type Float%20%28single-precision%29))
  (bind _ns_beam (Variables|Default|GetNS_Beam))
  (Niagara|SetNiagaraVariable(Vector3) _ns_beam "EndPos" (Math|Vector|MakeVector (Math|Vector|VectorLength (- (Transformation|GetWorldLocation (Variables|Default|GetEndPoint)) (Transformation|GetWorldLocation _ns_beam))) 0.0 0.0)))

(event Input|KeyboardEvents|R
  (params (Key :type Key%20Structure :default "None"))
  (:Pressed
    (Class|Gun|Reload)))

(event Input|MouseEvents|ThumbMouseButton2
  (params (Key :type Key%20Structure :default "None"))
  (:Pressed
    (Class|Gun|Shoot)))

(fn ConstructionScript)