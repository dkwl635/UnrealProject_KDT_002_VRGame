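; BP_ForestGhost is a monster actor that relocates across the map when it stays in light too long or takes successful damage.
; Capsule overlaps with Light-type objects call begin/end light handlers and set a flag, starting a short countdown on entry that Tick runs down.
; When the countdown expires or damage lands, RandomSpawn waits briefly, then teleports the ghost to a random XY within fixed bounds, keeping its height.
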(event OnComponentBeginOverlap(CapsuleComponent)
  (params (OverlappedComponent :type Primitive%20Component%20Object%20Reference) (OtherActor :type Actor%20Object%20Reference) (OtherComp :type Primitive%20Component%20Object%20Reference) (OtherBodyIndex :type Integer) (bFromSweep :type Boolean) (SweepResult :type Hit%20Result%20Structure%20%28by%20ref%29))
  (switch Utilities|FlowControl|Switch|SwitchonECollisionChannel (Collision|GetCollisionObjectType OtherComp)
    (:ECC_GameTraceChannel2
      (Class|ForestMonster|OnBeginLight)
      (Variables|Default|SetIsInLight true)
      (Variables|Default|SetLightTimer 2.0))))

(event OnComponentEndOverlap(CapsuleComponent)
  (params (OverlappedComponent :type Primitive%20Component%20Object%20Reference) (OtherActor :type Actor%20Object%20Reference) (OtherComp :type Primitive%20Component%20Object%20Reference) (OtherBodyIndex :type Integer))
  (switch Utilities|FlowControl|Switch|SwitchonECollisionChannel (Collision|GetCollisionObjectType OtherComp)
    (:ECC_GameTraceChannel2
      (Class|ForestMonster|OnEndLight)
      (Variables|Default|SetIsInLight false))))

(event Custom|RandomSpawn
  (Utilities|FlowControl|Delay 0.5)
  (Transformation|SetActorLocation (Math|Vector|MakeVector (Math|Random|RandomFloatinRange -8e+03 8e+03) (Math|Random|RandomFloatinRange -8e+03 8e+03) (.z (Transformation|GetActorLocation))) false true))

(event EventTakeSuccessDamage
  (CallFunction|RandomSpawn))

(event EventTick
  (params (DeltaSeconds :type Float%20%28single-precision%29))
  (if (Variables|Default|GetIsInLight)
    (bind _output_get (Variables|Default|SetLightTimer (- (Variables|Default|GetLightTimer) DeltaSeconds)))
    (if (<= _output_get 0.0)
      (Variables|Default|SetIsInLight false)
      (CallFunction|RandomSpawn))))

(fn ConstructionScript)