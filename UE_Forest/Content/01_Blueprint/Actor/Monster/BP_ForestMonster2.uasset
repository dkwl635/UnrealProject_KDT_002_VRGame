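; Forest monster actor Blueprint that handles the creature's spawn and death visuals.
; On BeginPlay, extra meshes follow the main skeletal mesh via leader pose, step audio starts, and body, hair and tail get dynamic materials.
; Damage plays the death montage and starts a one-second Tick countdown that drives paper-burn and dissolve parameters, then switches MF_Disable as it ends.
; The spawn event resets those parameters, restoring the look without recreating materials.
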(event EventBeginPlay
  (Components|SkinnedMesh|SetLeaderPoseComponent (Variables|Default|GetSkeletalMesh1) (Variables|Default|GetSkeletalMeshComponent) false false)
  (Audio|Components|Audio|Play (Variables|Default|GetStepAudioComponent) 0.0)
  (bind _returnvalue (Rendering|Material|CreateDynamicMaterialInstance (Variables|Default|GetSkeletalMeshComponent) 0 0 "None" :!class /Script/Engine.PrimitiveComponent))
  (Variables|Default|SetBodyMt _returnvalue)
  (bind _returnvalue_2 (Rendering|Material|CreateDynamicMaterialInstance (Variables|Default|GetSkeletalMesh) 0 0 "None" :!class /Script/Engine.PrimitiveComponent))
  (Variables|Default|SetHairMt _returnvalue_2)
  (bind _returnvalue_3 (Rendering|Material|CreateDynamicMaterialInstance (Variables|Default|GetSkeletalMesh1) 0 0 "None" :!class /Script/Engine.PrimitiveComponent))
  (Variables|Default|SetTailVar _returnvalue_3))

(event EventTakeDamageEvent
  (Animation|Montage|MontagePlay (Variables|Default|GetMonsterAnimInstance) "/Game/02_Animation/ForestMonster/ForestMonster2/ForestMonster2_Die_Montage.ForestMonster2_Die_Montage" 1.0 "Duration" 0.0 true)
  (Variables|Default|SetDieTimer 1.0))

(event EventTick
  (params (DeltaSeconds :type Float%20%28single-precision%29))
  (if (> (Variables|Default|GetDieTimer) 0.0)
    (bind _output_get (Variables|Default|SetDieTimer (- (Variables|Default|GetDieTimer) DeltaSeconds)))
    (if (< _output_get 0.1)
      (Rendering|Material|SetScalarParameterValue (Variables|Default|GetBodyMt) "MF_Disable" 0.0 :!class /Script/Engine.MaterialInstanceDynamic)
      (else
        (Rendering|Material|SetScalarParameterValue (Variables|Default|GetBodyMt) "MF_PostEffect_PaperBurn" _output_get :!class /Script/Engine.MaterialInstanceDynamic)
        (Rendering|Material|SetScalarParameterValue (Variables|Default|GetBodyMt) "MF_PostEffect_Dissolve" _output_get :!class /Script/Engine.MaterialInstanceDynamic)))))

(event EventMonsterSpawnEvent
  (Rendering|Material|SetScalarParameterValue (Variables|Default|GetBodyMt) "MF_Disable" 1.0 :!class /Script/Engine.MaterialInstanceDynamic)
  (Rendering|Material|SetScalarParameterValue (Variables|Default|GetBodyMt) "MF_PostEffect_PaperBurn" 1.0 :!class /Script/Engine.MaterialInstanceDynamic)
  (Rendering|Material|SetScalarParameterValue (Variables|Default|GetBodyMt) "MF_PostEffect_Dissolve" 1.0 :!class /Script/Engine.MaterialInstanceDynamic))

(fn ConstructionScript)