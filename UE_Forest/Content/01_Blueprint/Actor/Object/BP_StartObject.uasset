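; BP_StartObject is the game start set piece, with a table, spotlight, child actors and a widget component hosting BPUI_GameStart.
; On BeginPlay it binds two handlers to that widget's start button and countdown end events.
; The button handler makes the two child actors visible, and the countdown handler hides the table, spotlight and widget.
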(event Custom|GameStartButtonFunction
  (Rendering|SetVisibility (Variables|Default|GetChildActor) true false))

(event Custom|GameStart
  (Rendering|SetVisibility (Variables|Default|GetTable) false false))

(event EventBeginPlay
  (bind _asbpui_game_start (Utilities|Casting|CastToBPUI_GameStart (UserInterface|GetWidget (Variables|Default|GetWidget))))
  (EventDispatchers|BindEventtoGameStartButtonFunction _asbpui_game_start (delegate Custom|GameStartButtonFunction))
  (EventDispatchers|BindEventtoGameCountDownEnd _asbpui_game_start (delegate Custom|GameStart)))

(event Collision|EventActorBeginOverlap
  (params (OtherActor :type Actor%20Object%20Reference)))

(event EventTick
  (params (DeltaSeconds :type Float%20%28single-precision%29)))

(fn ConstructionScript)